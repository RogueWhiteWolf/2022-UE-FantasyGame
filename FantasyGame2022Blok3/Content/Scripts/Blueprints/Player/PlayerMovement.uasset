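; Player character Blueprint handling walk, jump and crouch input, plus camera turning.
; Forward movement follows control yaw, strafing follows actor rotation, and Turn input yaws the CameraBoom directly.
; Tick eases controller yaw toward the input direction, weighted by input strength and how sideways it is, giving an automatic follow camera.
; Sword and look-up inputs are stubs; camera reset and the velocity-scaled AutoAdjustCam alternative are disconnected.
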(event `InputAction|UseSword`
  (params (Key :type "Key Structure"))
  ;[1 1 1] Weapons
  (:`Pressed`
    (if true
      _)))

(event `InputAction|FireBow`
  (params (Key :type "Key Structure"))
  ;[1 1 1] Weapons
)

(event `InputAction|Crouch`
  (params (Key :type "Key Structure"))
  ;[1 1 1] Character Actions
  (:`Pressed`
    (`self.Crouch`))
  (:`Released`
    (`self.UnCrouch`)))

(event `InputAxis|MoveForward` :overrideparent false
  (params (AxisValue :type "Float (single-precision)"))
  ;[1 1 1] Movement
  (`self.AddMovementInput` (`KismetMathLibrary.GetForwardVector` (`KismetMathLibrary.MakeRotator` 0.0 0.0 (.yaw (`self.GetControlRotation`)))) AxisValue))

(event `InputAction|Jump` :overrideparent false
  (params (Key :type "Key Structure"))
  ;[1 1 1] Character Actions
  (:`Pressed`
    (`self.Jump`))
  (:`Released`
    (`self.StopJumping`)))

(event `InputAxis|MoveRight` :overrideparent false
  (params (AxisValue :type "Float (single-precision)"))
  ;[1 1 1] Movement
  (`self.AddMovementInput` (`KismetMathLibrary.GetRightVector` (`self.K2_GetActorRotation` self)) AxisValue))

(event `InputAxis|Turn` :overrideparent false
  (params (AxisValue :type "Float (single-precision)"))
  (bind _camera_boom (`self.Camera Boom`))
  (bind (_returnvalue_roll _returnvalue_pitch _returnvalue_yaw) (`KismetMathLibrary.BreakRotator` (`SceneComponent.K2_GetComponentRotation` _camera_boom)))
  ;[1 1 1] Rotate Camera
  (`SceneComponent.K2_SetWorldRotation` _camera_boom (`KismetMathLibrary.MakeRotator` 0.0 0.0 (+ _returnvalue_yaw (* (`self.BaseTurnRate`) AxisValue))) false false))

(event `self.ReceiveTick`
  (params (DeltaSeconds :type "Float (single-precision)"))
  (bind _returnvalue (`KismetMathLibrary.MakeRotator` 0.0 0.0 (.yaw (`self.GetControlRotation`))))
  (bind _returnvalue_2 (`KismetMathLibrary.Normal` (+ (* (`KismetMathLibrary.GetForwardVector` _returnvalue) (`self.GetInputAxisValue`)) (* (`KismetMathLibrary.GetRightVector` _returnvalue) (`self.GetInputAxisValue`)))))
  (`self.AddControllerYawInput` (* (`KismetMathLibrary.FClamp` (* DeltaSeconds (`KismetMathLibrary.FClamp` (+ (`KismetMathLibrary.Abs` (`self.GetInputAxisValue`)) (`KismetMathLibrary.Abs` (`self.GetInputAxisValue`)))) (`KismetMathLibrary.MultiplyMultiply_FloatFloat` (- 1.0 (`KismetMathLibrary.Abs` (`KismetMathLibrary.Dot_VectorVector` (`KismetMathLibrary.GetForwardVector` (`KismetMathLibrary.MakeRotator` 0.0 0.0 (.yaw (`self.GetControlRotation`)))) _returnvalue_2))) 0.5))) (.yaw (`KismetMathLibrary.NormalizedDeltaRotator` (`KismetMathLibrary.Conv_VectorToRotator` _returnvalue_2) (`self.GetControlRotation`))))))

(event `InputAxis|LookUp` :overrideparent false
  (params (AxisValue :type "Float (single-precision)"))
  ;[1 1 1] Rotate Camera
)

(event `InputAction|ResetCamera`
  (params (Key :type "Key Structure"))
  ;[1 1 1] Reset Camera
)

(fn `AutoAdjustCam`
  (locals (yInput :type "Float (double-precision)") (NewLocalVar_0 :type Boolean :default false))
  (bind (_returnvalue_x _returnvalue_y) (`KismetMathLibrary.BreakVector` (`self.GetVelocity`)))
  (bind _yinput (`local.yInput`))
  (bind (_returnvalue_x_2 _returnvalue_y_2) (`KismetMathLibrary.BreakVector` (`KismetMathLibrary.Normal` (`KismetMathLibrary.MakeVector` (`self.GetInputAxisValue`) (`self.GetInputAxisValue`)))))
  (bind _output_get (set `local.yInput` _returnvalue_y_2))
  (if (!= _output_get 0.0)
    (`self.AddControllerYawInput` (* (* _yinput (`KismetMathLibrary.MultiplyMultiply_FloatFloat` (`KismetMathLibrary.Abs` _yinput) (`self.camAngleExponent`))) 100.0 (/ (`KismetMathLibrary.VSize` (`KismetMathLibrary.MakeVector` _returnvalue_x _returnvalue_y)) (`self.basePlayerWalkSpeed`)) (`self.camRotationFactor`) (`GameplayStatics.GetWorldDeltaSeconds`)))))

(fn `UserConstructionScript`)